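; Gameplay ability that watches its owner's health attribute and triggers death when it runs out.
; On activation, an async task listens for attribute changes on the owner's Ability System Component, passing each new value to an optional debug print.
; At zero or below, it activates abilities by the Death gameplay tag, allowing remote activation, so death logic stays in a separate ability.
; The stored task is ended when the ability ends.
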(event Ability|EventActivateAbility
  (bind (_asynctaskproxy _attribute _newvalue) (|ListenforAttributeChange (Ability|GetAbilitySystemComponentfromActorInfo) "(AttributeName=\"Health\",Attribute=/Script/WarGAS.CC_AttributeSet:Health,AttributeOwner=\"/Script/CoreUObject.Class'/Script/WarGAS.CC_AttributeSet'\")")
    (:then
      (Variables|Default|SetAttributeChangeTask _asynctaskproxy))
    (:OnAttributeChanged
      (CallFunction|DebugPrintNewHealth _newvalue)
      (if (<= _newvalue 0.0)
        ;[0.15 0.15 0.15 0.5] Activator ability by tag
        (Abilities|TryActivateAbilitiesbyTag (Ability|GetAbilitySystemComponentfromActorInfo) (GameplayTags|MakeGameplayTagContainerfromTag (GameplayTags|MakeLiteralGameplayTag "(TagName=\"CCTags.CCAbilities.Death\")")) true)))))

(event Ability|EventOnEndAbility
  (params (bWasCancelled :type Boolean))
  (bind _attributechangetask (Variables|Default|GetAttributeChangeTask)
    (:then
      (Class|CCAttributeChangeTask|EndTask _attributechangetask))
    (:else)))

(fn DebugPrintNewHealth
  (params (InDouble :type Float%20%28double-precision%29))
  (Variables|Default|GetbDrawDebugs
    (:then
      (Development|PrintString (Utilities|String|Append "GA_CC_ListenForHealthChange:  " (Utilities|GetDisplayName (Ability|GetAvatarActorfromActorInfo)) "New Health Value: " (Utilities|String|ToString(Float) InDouble))))
    (:else)))