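; GA_CC_HitReact is an enemy gameplay ability that plays a directional hit reaction montage.
; On activation it waits for the HitReact gameplay event and skips the reaction if the owner has the Dead tag.
; Otherwise C++ helpers compute the hit direction from the avatar's forward and the instigator, and the montage jumps to the section named after that direction.
; Print-string debugging reports the tag check, event source and direction.
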(event Ability|EventActivateAbility
  (bind _payload (Ability|Tasks|WaitGameplayEvent "(TagName=\"CCTags.Events.Enemy.HitReact\")" 0)
    (:EventReceived
      (if (GameplayTags|HasMatchingGameplayTag (Ability|GetAbilitySystemComponentfromActorInfo) "(TagName=\"CCTags.Status.Dead\")")
        (Development|PrintString "Has Matching Gameplay Tag: TRUE" true true "(R=0.091017,G=0.541667,B=0.059810,A=1.000000)")
        (else
          (Development|PrintString "Has Matching Gameplay Tag: FALSE" true true "(R=0.286458,G=0.000125,B=0.033818,A=1.000000)")
          (CallFunction|PrintDebugEventReceived _payload)
          ;[1 0.8789 0 0.5] This created in C++
          (Class|CCHitReact|CacheHitDirectionVectors (.Instigator (Utilities|Struct|BreakGameplayEventData _payload)))
          (Utilities|FlowControl|Sequence
            (:then_0
              ;[1 0.8789 0 0.5] This created in C++ - Cache Hit Direction Name
              (Variables|Default|SetDirectionName (Class|CCBlueprintLibrary|GetHitDirectionName (Class|CCBlueprintLibrary|GetHitDirection (Variables|Default|GetAvatarForward) (Variables|Default|GetToInstigator))))
              ;[0.8789 0 0.3264 0.5] Debug for Direction
              (Variables|Default|GetbDrawDebugs
                (:then
                  (Development|PrintString (Utilities|String|ToString(Name) (Variables|Default|GetDirectionName)) true true "(R=0.114583,G=0.000000,B=0.075680,A=1.000000)"))
                (:else)))
            (:then_1
              (|PlayMontageandWaitProxy "None" (Variables|Default|GetHitReactMontage) 1.0 "None" true 1.0 0.0 false
                (:then
                  (Ability|Animation|MontageJumptoSection (Variables|Default|GetDirectionName)))))))))))

(fn PrintDebugEventReceived
  (params (GameplayEventData :type Gameplay%20Event%20Data%20Structure%20%28by%20ref%29))
  (Variables|Default|GetbDrawDebugs
    (:then
      (Development|PrintString (Utilities|String|Append "GA_CC_HitReact_Received_Event_From" (Utilities|GetDisplayName (.Instigator (Utilities|Struct|BreakGameplayEventData GameplayEventData)))) true true "(R=0.276099,G=0.000000,B=0.364583,A=1.000000)"))
    (:else)))