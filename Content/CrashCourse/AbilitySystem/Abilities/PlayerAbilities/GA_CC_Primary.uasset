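; Gameplay Ability for the player's primary attack in CrashCourse, dealing damage to actors caught in a hit box.
; Each activation uses a FlipFlop to pick attack montage A or B, ending the ability when the montage finishes or is interrupted.
; A Player.Primary gameplay event runs the C++ hit box overlap test, sends hit reacts and applies GE_PlayerDamage to each actor found.
; The debug sphere drawing is not connected.
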(event Ability|EventActivateAbility
  (bind _returnvalue (Ability|GetAbilitySystemComponentfromActorInfo))
  (Utilities|FlowControl|Sequence
    (:then_0
      (Utilities|FlowControl|FlipFlop
        (:A
          ;[0.984 1 0.9559] Play Attack Montage
          (|PlayMontageandWaitProxy "None" "/Game/CrashCourse/Animations/Player/AnimMontage/Primary_A_Montage.Primary_A_Montage" 1.0 "None" true 1.0 0.0 false
            (:OnCompleted
              _)
            (:OnBlendOut
              _)
            (:OnInterrupted
              _)
            (:OnCancelled
              _))
          (Ability|EndAbility))
        (:B
          (|PlayMontageandWaitProxy "None" "/Game/CrashCourse/Animations/Player/AnimMontage/Primary_B_Montage.Primary_B_Montage" 1.0 "None" true 1.0 0.0 false
            (:OnCompleted
              _)
            (:OnBlendOut
              _)
            (:OnInterrupted
              _)
            (:OnCancelled
              _))
          (Ability|EndAbility))))
    (:then_1
      (Ability|Tasks|WaitGameplayEvent "(TagName=\"CCTags.Events.Player.Primary\")" 0
        (:EventReceived
          ;[1 0.8789 0 0.5] This created in C++
          (bind _returnvalue_2 (Class|CCPrimary|HitBoxOverlapTest))
          (Class|CCPrimary|SendHitReactEventtoActors _returnvalue_2)
          (for _array_element _returnvalue_2
            (GameplayEffects|ApplyGameplayEffectSpecToTarget _returnvalue (GameplayEffects|MakeOutgoingSpec :self _returnvalue :GameplayEffectClass "/Game/CrashCourse/AbilitySystem/GameplayEffects/Player/GE_PlayerDamage.GE_PlayerDamage_C" :Level 1.0) (Ability|GetAbilitySystemComponent _array_element))))))))

(event Ability|EventOnEndAbility
  (params (bWasCancelled :type Boolean))
  (if (Variables|Default|GetbDrawDebugs)
    (Development|PrintString "GA_Primary: End")))